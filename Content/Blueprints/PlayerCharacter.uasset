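; Player character Blueprint that moves, turns and shoots through Enhanced Input, registering its mapping context on the controller's local player subsystem at BeginPlay.
; Move applies movement input along the actor's right vector only, and Rotate adds yaw scaled by RotationSpeed without delta time.
; Shoot delegates to the WeaponPewPewLaser's TryShoot.
; The TakeDamage event destroys the actor outright, with no health check.
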(event Input|EnhancedActionEvents|EnhancedInputActionMove
  (params (ActionValue :type Float%20%28double-precision%29) (ElapsedSeconds :type Float%20%28double-precision%29) (TriggeredSeconds :type Float%20%28double-precision%29) (InputAction :type Input%20Action%20Object%20Reference :default "/Game/Inputs/Move.Move"))
  (Pawn|Input|AddMovementInput (Transformation|GetActorRightVector) ActionValue false))

(event Input|EnhancedActionEvents|EnhancedInputActionRotate
  (params (ActionValue :type Float%20%28double-precision%29) (ElapsedSeconds :type Float%20%28double-precision%29) (TriggeredSeconds :type Float%20%28double-precision%29) (InputAction :type Input%20Action%20Object%20Reference :default "/Game/Inputs/Rotate.Rotate"))
  (Class|Actor|AddActorWorldRotation (Math|Rotator|MakeRotator 0.0 0.0 (* ActionValue (Variables|Default|GetRotationSpeed)))))

(event Input|EnhancedActionEvents|EnhancedInputActionShoot
  (params (ActionValue :type Boolean) (ElapsedSeconds :type Float%20%28double-precision%29) (TriggeredSeconds :type Float%20%28double-precision%29) (InputAction :type Input%20Action%20Object%20Reference :default "/Game/Inputs/Shoot.Shoot"))
  (Default|TryShoot (Variables|Default|GetWeaponPewPewLaser)))

(event EventBeginPlay
  (bind _asplayer_controller (Utilities|Casting|CastToPlayerController (Pawn|GetController)))
  (Utilities|IsValid (PlayerController|LocalPlayerSubsystems|GetEnhancedInputLocalPlayerSubsystem _asplayer_controller)
    (:Is%20Valid
      (Input|AddMappingContext (PlayerController|LocalPlayerSubsystems|GetEnhancedInputLocalPlayerSubsystem _asplayer_controller) "/Game/Inputs/PlayerInputMapping.PlayerInputMapping" 0 "(bIgnoreAllPressedKeysUntilRelease=True,bForceImmediately=False,bNotifyUserSettings=False)"))))

(event Collision|EventActorBeginOverlap
  (params (OtherActor :type Actor%20Object%20Reference)))

(event EventTick
  (params (DeltaSeconds :type Float%20%28single-precision%29)))

(event EventTakeDamage
  (params (Amount :type Float%20%28double-precision%29))
  (Actor|DestroyActor))

(fn ConstructionScript)