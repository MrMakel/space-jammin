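; Base weapon Blueprint that fires projectiles with a minimum delay between shots.
; TryShoot calls Shoot only when the time since LastShotTime exceeds ShotDelay.
; Shoot spawns ProjectileClass at the owner's actor transform, then records the game time as LastShotTime.
; BeginPlay and Tick are empty, so firing depends on external calls.
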(event EventBeginPlay)

(event EventTick
  (params (DeltaSeconds :type Float%20%28single-precision%29)))

(fn Shoot
  (Game|SpawnActorfromClass (Variables|Properties|GetProjectileClass) (Transformation|GetActorTransform (Components|GetOwner)) "Undefined" "MultiplyWithRoot" 0 0)
  (Variables|Default|SetLastShotTime (Utilities|Time|GetGameTimeinSeconds)))

(fn TryShoot
  (if (> (- (Utilities|Time|GetTimeSeconds) (Variables|Default|GetLastShotTime)) (Variables|Properties|GetShotDelay))
    (CallFunction|Shoot)))