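; Base projectile actor for weapons, moved by a ProjectileMovement component.
; The construction script sets its velocity along local +Y, scaled by Speed.
; On overlap it destroys itself, except that shots not flagged IsEnemyShot pass through PlayerCharacter actors.
; It applies no damage or effects.
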(event EventBeginPlay)

(event Collision|EventActorBeginOverlap
  (params (OtherActor :type Actor%20Object%20Reference))
  (if (Utilities|ClassIsChildOf (Utilities|GetClass OtherActor) "/Game/Blueprints/PlayerCharacter.PlayerCharacter_C")
    (if (Variables|Default|GetIsEnemyShot)
      (Actor|DestroyActor :!label _label))
    (else
      (goto _label))))

(event EventTick
  (params (DeltaSeconds :type Float%20%28single-precision%29)))

(fn ConstructionScript
  (Game|Components|ProjectileMovement|SetVelocityinLocalSpace (Variables|Default|GetProjectileMovement) (* "0.000000,1.000000,0.000000" (Variables|Properties|GetSpeed))))